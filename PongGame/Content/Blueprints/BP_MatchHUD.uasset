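; BP_MatchHUD is a HUD Blueprint that draws a vertical dashed line down the horizontal center of the screen.
; DrawHUD loops over LineCount to draw evenly spaced segments from the length, spacing and color variables, plus a "0" text each pass.
; The vertical offset is a sine of frame delta time times LineMovementSpeed, scaled by half the viewport height, so it follows frame time rather than elapsed time.
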(event `self.ReceiveDrawHUD`
  (params (SizeX :type Integer) (SizeY :type Integer))
  (bind (_returnvalue_x _returnvalue_y) (`KismetMathLibrary.BreakVector2D` (`WidgetLayoutLibrary.GetViewportSize`)))
  (bind _linecolor (`self.LineColor`))
  (bind _returnvalue (`KismetMathLibrary.Conv_IntToDouble` (/ SizeX 2)))
  (set `self.CurrentOffset` (* (`KismetMathLibrary.Sin` (* (`GameplayStatics.GetWorldDeltaSeconds`) (`self.LineMovementSpeed`))) (/ _returnvalue_y 2.0)))
  (for _index (range (+ (`self.LineCount`) 1))
    (bind _returnvalue_2 (+ (`self.CurrentOffset`) (* _index (+ (`self.LineLenght`) (`self.LineSpacing`)))))
    (`self.DrawLine` _returnvalue _returnvalue_2 _returnvalue (+ _returnvalue_2 (`self.LineLenght`)) _linecolor 2.0)
    (`self.DrawText` "0" _linecolor 0.0 0.0 null)))

(fn `UserConstructionScript`)