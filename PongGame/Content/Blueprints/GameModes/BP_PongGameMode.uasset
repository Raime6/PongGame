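; Game mode for a Pong match that handles ball spawning and the win condition.
; BeginPlay caches all paddles as players and spawns a ball after a short delay at a random Y on the center line.
; UpdatePlayerScore checks paddle scores against WinScore, then copies names, scores and CurrentWinner into GI_MatchInfo.
; The game instance carries these results into the EndGame level it opens.
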(event `self.ReceiveBeginPlay`
  (bind _outactors (`GameplayStatics.GetAllActorsOfClass` "/Game/Blueprints/BP_Paddle.BP_Paddle_C"))
  (set `self.Player` _outactors)
  (`self.Spawn Ball`))

(event `Spawn Ball`
  ;[0.05098 0.05098 0.05098] Spawn Ball
  (`KismetSystemLibrary.Delay` 2.7)
  (`|SpawnActorFromClass` "/Game/Blueprints/BP_Ball.BP_Ball_C" (`KismetMathLibrary.Conv_VectorToTransform` (`KismetMathLibrary.MakeVector` 0.0 (`KismetMathLibrary.RandomFloatInRange` -82.0 82.0) 3.0)) "Undefined" "MultiplyWithRoot" null null))

(event `Update PlayerScore`
  (for _array_element (`self.Player`)
    (if (== (`/Game/Blueprints/BP_Paddle.Score` _array_element) (`self.Win_Score`))
      (bind _asgi_match_info (cast `/Game/Blueprints/GameInstances/GI_MatchInfo` (`GameplayStatics.GetGameInstance`)))
      (set `self.GameInstance` _asgi_match_info)
      (for (_array_element_2 _array_index) (`self.Player`)
        (`KismetArrayLibrary.Array_Set` (`/Game/Blueprints/GameInstances/GI_MatchInfo.PlayerNames` (`self.GameInstance`)) _array_index (`/Game/Blueprints/BP_Paddle.Player_Name` _array_element_2) true)
        (`KismetArrayLibrary.Array_Set` (`/Game/Blueprints/GameInstances/GI_MatchInfo.Scores` (`self.GameInstance`)) _array_index (`/Game/Blueprints/BP_Paddle.Score` _array_element_2) true))
      (set `/Game/Blueprints/GameInstances/GI_MatchInfo.Winner` (`self.Current_Winner`) (`self.GameInstance`))
      (`GameplayStatics.OpenLevel` "EndGame"))))

(fn `UserConstructionScript`)