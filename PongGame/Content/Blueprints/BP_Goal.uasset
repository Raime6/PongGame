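; BP_Goal is a Pong goal that awards a point to its linked MyPlayer when a BP_Ball overlaps it.
; On overlap it destroys the ball, increments that player's score and calls UpdatePlayerScore on BP_Pong_GameMode.
; It sets the game mode's CurrentWinner to the opposite PlayerSelection value from MyPlayer's.
; It writes the score to the matching field on the first BP_MatchHUD found, then asks the game mode to spawn a new ball.
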(event `self.ReceiveActorBeginOverlap`
  (params (OtherActor :type "Actor Object Reference"))
  (bind _player_selection (`/Game/Blueprints/BP_Paddle.Player_Selection` (`self.MyPlayer`)))
  (bind _score (`/Game/Blueprints/BP_Paddle.Score` (`self.MyPlayer`)))
  (bind _asbp_ball (cast `/Game/Blueprints/BP_Ball` OtherActor))
  (`self.K2_DestroyActor` _asbp_ball)
  (`/Engine/EditorBlueprintResources/StandardMacros.IncrementInt` _score
    (:`  `
      (bind _asbp_pong_game_mode (cast `/Game/Blueprints/BP_Pong_GameMode` (`GameplayStatics.GetGameMode`)))
      (`/Game/Blueprints/BP_Pong_GameMode.Update PlayerScore` _asbp_pong_game_mode)
      ;[0.05098 0.05098 0.05098] Updates the last point winner
      (if (`|EnumEquality` _player_selection "NewEnumerator0")
        (set `/Game/Blueprints/BP_Pong_GameMode.Current_Winner` "NewEnumerator1" _asbp_pong_game_mode)
        (else
          (set `/Game/Blueprints/BP_Pong_GameMode.Current_Winner` "NewEnumerator0" _asbp_pong_game_mode)))
      (bind _outactors (`GameplayStatics.GetAllActorsOfClass` "/Game/Blueprints/BP_MatchHUD.BP_MatchHUD_C"))
      (if (`|EnumEquality` _player_selection "NewEnumerator0")
        (bind _output (`|GetArrayItem` _outactors))
        (set `/Game/Blueprints/BP_MatchHUD.Player1Score` _score _output)
        (else
          (set `/Game/Blueprints/BP_MatchHUD.Player2Score` _score _output)))
      ;[0.05098 0.05098 0.05098] Spawns the Ball
      (bind _asbp_pong_game_mode_2 (cast `/Game/Blueprints/BP_Pong_GameMode` (`GameplayStatics.GetGameMode`)))
      (`/Game/Blueprints/BP_Pong_GameMode.Spawn Ball` _asbp_pong_game_mode_2))))

(fn `UserConstructionScript`)