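; Pong paddle Blueprint that either Player 1 or Player 2 moves, chosen by its PlayerSelection variable.
; BeginPlay adds the IMC_Player1 mapping context and enables input from player controller 0.
; Each player's Enhanced Input movement action calls MoveRaquet only on the matching paddle.
; MoveRaquet scales input by speed and frame time into a clamped alpha, placing the mesh by Lerp between actors A and B.
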(event `self.ReceiveBeginPlay`
  (bind _returnvalue (pcsubsystem `EnhancedInputLocalPlayerSubsystem` (`GameplayStatics.GetPlayerController` 0)))
  ;[1 1 1] Init Input
  (`/Engine/EditorBlueprintResources/StandardMacros.IsValid` _returnvalue
    (:`Is Valid`
      (`EnhancedInputSubsystemInterface.AddMappingContext` _returnvalue "/Game/Input/IMC_Player1.IMC_Player1" 0 (struct))
      (`self.EnableInput` (`GameplayStatics.GetPlayerController` 0)))))

(event `Move Raquet`
  (params (Quantity :type "Float (double-precision)"))
  ;[1 1 1] Interpola la posición del objeto entre A y B
  (set `self.C` (`KismetMathLibrary.FClamp` (+ (* Quantity (`GameplayStatics.GetWorldDeltaSeconds`) (`self.Speed`)) (`self.C`))))
  (`SceneComponent.K2_SetWorldLocation` (`self.StaticMeshComponent`) (`KismetMathLibrary.VLerp` (`self.K2_GetActorLocation` (`self.A`)) (`self.K2_GetActorLocation` (`self.B`)) (`self.C`)) false false))

(event `EnhancedInput|/Game/Input/Input_Movement_Player1`
  (params (ActionValue :type "Float (double-precision)") (ElapsedSeconds :type "Float (double-precision)") (TriggeredSeconds :type "Float (double-precision)") (InputAction :type "InputAction Object Reference" :default "/Game/Input/Input_Movement_Player1.Input_Movement_Player1"))
  ;[1 1 1] Move Raquet
  (:`Triggered`
    (switch `/Game/Blueprints/Player_Type` (`self.Player_Selection`)
      (:`NewEnumerator0`
        (`self.Move Raquet` ActionValue)))))

(event `EnhancedInput|/Game/Input/Input_Movement_Player2`
  (params (ActionValue :type "Float (double-precision)") (ElapsedSeconds :type "Float (double-precision)") (TriggeredSeconds :type "Float (double-precision)") (InputAction :type "InputAction Object Reference" :default "/Game/Input/Input_Movement_Player2.Input_Movement_Player2"))
  ;[1 1 1] Move Raquet
  (:`Triggered`
    (switch `/Game/Blueprints/Player_Type` (`self.Player_Selection`)
      (:`NewEnumerator1`
        (`self.Move Raquet` ActionValue)))))

(fn `UserConstructionScript`)