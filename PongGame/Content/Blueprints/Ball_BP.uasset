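; Physics-driven ball that launches toward a target actor and bounces at constant speed, counting rebounds and adding a HUD widget on start.
; Each hit reflects Direction off the normal impulse, then passes it through four per-quadrant Watch checks before reapplying linear velocity.
; The checks rotate headings near ±90 degrees 10 degrees away from that axis, using configurable angle limits.
; Overlaps only print the other actor's name, and NewFunction is never called.
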(event `self.ReceiveBeginPlay`
  ;[1 1 1] Init
  (`PrimitiveComponent.SetSimulatePhysics` (`self.StaticMeshComponent`) true)
  (`self.Calculate Initial Direction`)
  (`self.Calculate Impulse`)
  (bind _returnvalue (`|CreateWidget` "/Game/Blueprints/My_Widget_BP.My_Widget_BP_C" (`GameplayStatics.GetPlayerController` 0)))
  (`UserWidget.AddToViewport` _returnvalue 0))

(event `Calculate Initial Direction`
  ;[1 1 1] Set Direction
  (set `self.Direction` (`KismetMathLibrary.Normal` (- (`self.K2_GetActorLocation` (`self.Target Inicial`)) (`self.K2_GetActorLocation` self)))))

(event `Calculate Impulse`
  ;[1 1 1] Set Impulse
  (`PrimitiveComponent.SetPhysicsLinearVelocity` (`self.StaticMeshComponent`) (* (`self.Direction`) (`self.Velocity`)) false "None"))

(event `self.StaticMeshComponent.OnComponentHit`
  (params (HitComponent :type "PrimitiveComponent Object Reference") (OtherActor :type "Actor Object Reference") (OtherComp :type "PrimitiveComponent Object Reference") (NormalImpulse :type "Vector Structure") (Hit :type "HitResult Structure (by ref)"))
  ;[1 1 1] Calcula el reflejo y lanza la pelota en esa dirección
  (`/Engine/EditorBlueprintResources/StandardMacros.IncrementInt` (`self.Num Rebounds`)
    (:`  `
      (bind _output_get (set `self.Direction` (`KismetMathLibrary.Normal` (`KismetMathLibrary.GetReflectionVector` (`self.Direction`) NormalImpulse))))
      (bind _returnvalue (`KismetMathLibrary.RadiansToDegrees` (`KismetMathLibrary.Vector_HeadingAngle` _output_get)))
      ;;[1 1 1] Comprueba los ángulos de rebote y los modifica si fuese necesario
      (if (and (> _returnvalue (`self.Forward Max`)) (< _returnvalue 90.0))
        (bind _output_get_2 (set `self.Direction` (`KismetMathLibrary.RotateAngleAxis` (`self.Direction`) -10.0 (0.0 0.0 1.0)))))
      (bind _returnvalue_2 (`KismetMathLibrary.RadiansToDegrees` (`KismetMathLibrary.Vector_HeadingAngle` _output_get_2)))
      (if (and (> _returnvalue_2 90.0) (< _returnvalue_2 (`self.Backward Max`)))
        (bind _output_get_3 (set `self.Direction` (`KismetMathLibrary.RotateAngleAxis` (`self.Direction`) 10.0 (0.0 0.0 1.0)))))
      (bind _returnvalue_3 (`KismetMathLibrary.RadiansToDegrees` (`KismetMathLibrary.Vector_HeadingAngle` _output_get_3)))
      (if (and (> _returnvalue_3 -90.0) (< _returnvalue_3 (`self.Forward Min`)))
        (bind _output_get_4 (set `self.Direction` (`KismetMathLibrary.RotateAngleAxis` (`self.Direction`) 10.0 (0.0 0.0 1.0)))))
      (bind _returnvalue_4 (`KismetMathLibrary.RadiansToDegrees` (`KismetMathLibrary.Vector_HeadingAngle` _output_get_4)))
      (if (and (> _returnvalue_4 (`self.Backward Min`)) (< _returnvalue_4 -90.0))
        (set `self.Direction` (`KismetMathLibrary.RotateAngleAxis` (`self.Direction`) -10.0 (0.0 0.0 1.0))))
      (`self.Calculate Impulse`))))

(event `self.StaticMeshComponent.OnComponentBeginOverlap`
  (params (OverlappedComponent :type "PrimitiveComponent Object Reference") (OtherActor :type "Actor Object Reference") (OtherComp :type "PrimitiveComponent Object Reference") (OtherBodyIndex :type Integer) (bFromSweep :type Boolean) (SweepResult :type "HitResult Structure (by ref)"))
  (`KismetSystemLibrary.PrintString` (`KismetSystemLibrary.GetDisplayName` OtherActor)))

(fn `NewFunction`
  (params (A :type "Vector Structure"))
  (bind _returnvalue (`KismetMathLibrary.RadiansToDegrees` (`KismetMathLibrary.Vector_HeadingAngle` A)))
  (if (and (> _returnvalue 90.0) (< _returnvalue (`self.Backward Max`)))
    (set `self.Direction` (`KismetMathLibrary.RotateAngleAxis` (`self.Direction`) -10.0 (0.0 0.0 1.0)))))

(fn `UserConstructionScript`)