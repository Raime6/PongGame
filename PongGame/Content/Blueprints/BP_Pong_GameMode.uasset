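; Game mode for a Pong match that spawns the ball and ends the game when a paddle reaches the winning score.
; On BeginPlay it caches all paddle actors and spawns a ball at a random Y position.
; UpdatePlayerScore checks each paddle's score against WinScore.
; On a win it writes every paddle's score to a Match_Info save in the "Pong Score" slot, then opens Map_02.
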(event `self.ReceiveBeginPlay`
  (bind _outactors (`GameplayStatics.GetAllActorsOfClass` "/Game/Blueprints/BP_Paddle.BP_Paddle_C"))
  (set `self.Player` _outactors)
  (`self.Spawn Ball`))

(event `Spawn Ball`
  ;[0.05098 0.05098 0.05098] Spawn Ball
  (`|SpawnActorFromClass` "/Game/Blueprints/BP_Ball.BP_Ball_C" (`KismetMathLibrary.Conv_VectorToTransform` (`KismetMathLibrary.MakeVector` 0.0 (`KismetMathLibrary.RandomFloatInRange` -82.0 82.0) 3.0)) "Undefined" "MultiplyWithRoot" null null))

(event `Update PlayerScore`
  (for _array_element (`self.Player`)
    (if (== (`/Game/Blueprints/BP_Paddle.Score` _array_element) (`self.Win_Score`))
      (bind _returnvalue (`GameplayStatics.CreateSaveGameObject` "/Game/Blueprints/Match_Info.Match_Info_C"))
      (set `self.Current_Match` _returnvalue)
      (for _array_element_2 (`self.Player`)
        (`KismetArrayLibrary.Array_Add` (`/Game/Blueprints/Match_Info.Scores` (`self.Current_Match`)) (`/Game/Blueprints/BP_Paddle.Score` _array_element_2)))
      (`GameplayStatics.SaveGameToSlot` (`self.Current_Match`) "Pong Score")
      (`GameplayStatics.OpenLevel` "Map_02"))))

(fn `UserConstructionScript`)